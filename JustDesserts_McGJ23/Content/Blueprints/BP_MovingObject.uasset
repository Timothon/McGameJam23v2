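; Moving object actor that carries its MovingPoint between a start and an end location, such as for a platform or obstacle.
; A timeline at a configurable play rate drives a world-location lerp, reversing at each end to loop back and forth unless MoveOnce is set.
; Movement starts on BeginPlay or, with TriggeredStart, when the third-person character's capsule enters the collision box.
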(event OnComponentBeginOverlap(BoxCollision)
  (params (OverlappedComponent :type Primitive%20Component%20Object%20Reference) (OtherActor :type Actor%20Object%20Reference) (OtherComp :type Primitive%20Component%20Object%20Reference) (OtherBodyIndex :type Integer) (bFromSweep :type Boolean) (SweepResult :type Hit%20Result%20Structure%20%28by%20ref%29))
  (bind _asbp_third_person_character (Utilities|Casting|CastToBP_ThirdPersonCharacter OtherActor))
  (if (== (Variables|/Script/Engine.Character|GetCapsuleComponent _asbp_third_person_character) OtherComp)
    (if (Variables|Default|GetTriggeredStart)
      (CallFunction|StartMovement))))

(event Custom|StartMovement
  (bind _newtrack_0 (Timeline|MovementTimeline Play)
    (:Update
      (Transformation|SetWorldLocation (Variables|Default|GetMovingPoint) (Math|Vector|Lerp(Vector) (Transformation|GetWorldLocation (Variables|Default|GetStartLocation)) (Transformation|GetWorldLocation (Variables|Default|GetEndLocation)) _newtrack_0) false false))
    (:Finished
      (if (not (Variables|Default|GetMoveOnce))
        (if (== _newtrack_0 0.0)
          (CallFunction|StartMovement)
          (else
            (CallFunction|ReverseMovement)))))))

(event Custom|ReverseMovement
  (bind _newtrack_0 (Timeline|MovementTimeline Reverse)
    (:Update
      (Transformation|SetWorldLocation (Variables|Default|GetMovingPoint) (Math|Vector|Lerp(Vector) (Transformation|GetWorldLocation (Variables|Default|GetStartLocation)) (Transformation|GetWorldLocation (Variables|Default|GetEndLocation)) _newtrack_0) false false))
    (:Finished
      (if (not (Variables|Default|GetMoveOnce))
        (if (== _newtrack_0 0.0)
          (CallFunction|StartMovement)
          (else
            (CallFunction|ReverseMovement)))))))

(event EventBeginPlay
  (Components|Timeline|SetPlayRate (Variables|Default|GetMovementTimeline) (Variables|Default|GetPlayRate))
  (if (not (Variables|Default|GetTriggeredStart))
    (CallFunction|StartMovement)))

(event Collision|EventActorBeginOverlap
  (params (OtherActor :type Actor%20Object%20Reference)))

(event EventTick
  (params (DeltaSeconds :type Float%20%28single-precision%29)))

(fn ConstructionScript)