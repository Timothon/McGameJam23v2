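; Monster spawner manager that drops meteor-striking AI monsters into the level and configures collectibles.
; On BeginPlay it copies its PointSpawnInterval to every BP_CollectibleBase in the level.
; SpawnAtTargetPoint, not called within this Blueprint, spawns a BP_AIMonsterBase high above a randomly picked TargetPoint.
; It sets MeteorTarget from a random TargetPoint pick, then calls MeteorStrike on the new monster.
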(event EventBeginPlay
  (bind _outactors (Actor|GetAllActorsOfClass "/Game/Blueprints/BP_CollectibleBase.BP_CollectibleBase_C"))
  (for _array_element _outactors
    (Variables|/Game/Blueprints/BP_CollectibleBase.BP_CollectibleBase_C|SetPointSpawnInterval _array_element (Variables|Default|GetPointSpawnInterval))))

(event Collision|EventActorBeginOverlap
  (params (OtherActor :type Actor%20Object%20Reference)))

(event EventTick
  (params (DeltaSeconds :type Float%20%28single-precision%29)))

(fn ConstructionScript)

(fn SpawnatTargetPoint
  (bind _outactors (Actor|GetAllActorsOfClass "/Script/Engine.TargetPoint"))
  (bind _returnvalue (Game|SpawnActorfromClass "/Game/ThirdPerson/Blueprints/BP_AIMonsterBase.BP_AIMonsterBase_C" (Math|Transform|MakeTransform (+ (Transformation|GetActorLocation (.OutItem (Utilities|Array|Random _outactors))) "0,0,10000.000000") "0, 0, 0" "1.000000,1.000000,1.000000") "Undefined" 0 (Transformation|GetActorLocation (.OutItem (Utilities|Array|Random _outactors))) 0))
  (Default|MeteorStrike _returnvalue))