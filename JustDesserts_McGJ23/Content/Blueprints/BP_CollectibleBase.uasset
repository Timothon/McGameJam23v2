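; Base collectible pickup that adds points to the game instance's total and level scores when the player's capsule overlaps its sphere.
; Pickup shows a score widget, colour-tiered by value, which Tick floats upward and yaws toward the follow camera until the actor's delayed destruction.
; It also triggers all monster spawner managers when score outpaces monster count times an interval, below 30 monsters.
; CollectibleTaken is an empty hook called on pickup.
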(event OnComponentBeginOverlap(Sphere)
  (params (OverlappedComponent :type Primitive%20Component%20Object%20Reference) (OtherActor :type Actor%20Object%20Reference) (OtherComp :type Primitive%20Component%20Object%20Reference) (OtherBodyIndex :type Integer) (bFromSweep :type Boolean) (SweepResult :type Hit%20Result%20Structure%20%28by%20ref%29))
  (bind _scoregottenwidget (Variables|Default|GetScoreGottenWidget))
  (bind _pointsawarded (Variables|Default|GetPointsAwarded))
  (bind _asbp_third_person_character (Utilities|Casting|CastToBP_ThirdPersonCharacter OtherActor))
  (if (== (Variables|/Script/Engine.Character|GetCapsuleComponent _asbp_third_person_character) OtherComp)
    (bind _asbp_tpgame_instance (Utilities|Casting|CastToBP_TPGameInstance (Game|GetGameInstance)))
    (Variables|/Game/ThirdPerson/Blueprints/BP_TPGameInstance.BP_TPGameInstance_C|SetScore _asbp_tpgame_instance (+ (Variables|/Game/ThirdPerson/Blueprints/BP_TPGameInstance.BP_TPGameInstance_C|GetScore _asbp_tpgame_instance) (Variables|Default|GetPointsAwarded)))
    (Variables|/Game/ThirdPerson/Blueprints/BP_TPGameInstance.BP_TPGameInstance_C|SetCurrentLevelScore _asbp_tpgame_instance (+ (Variables|/Game/ThirdPerson/Blueprints/BP_TPGameInstance.BP_TPGameInstance_C|GetCurrentLevelScore _asbp_tpgame_instance) (Variables|Default|GetPointsAwarded)))
    (bind _asw_score_number (Utilities|Casting|CastToW_ScoreNumber (UserInterface|GetWidget _scoregottenwidget)))
    (Variables|/Game/Blueprints/UI/W_ScoreNumber.W_ScoreNumber_C|SetNumber _asw_score_number (Utilities|Text|ToText(Integer) _pointsawarded))
    (Rendering|SetVisibility _scoregottenwidget true false)
    (Transformation|SetWorldLocation _scoregottenwidget (+ (Transformation|GetWorldLocation (Variables|Default|GetSphere)) "0,0,20.000000") false false)
    (Variables|/Game/Blueprints/UI/W_ScoreNumber.W_ScoreNumber_C|SetTextColour _asw_score_number (select (< _pointsawarded 49) "(R=1.000000,G=1.000000,B=1.000000,A=1.000000)" (select (< _pointsawarded 99) "(R=0.000000,G=0.978051,B=1.000000,A=1.000000)" (select (< _pointsawarded 249) "(R=1.000000,G=0.000000,B=0.997644,A=1.000000)" "(R=1.000000,G=0.664949,B=0.000000,A=1.000000)"))))
    (CallFunction|SpawnMonsterDetection)
    (Components|DestroyComponent (Variables|Default|GetSphere))
    (CallFunction|CollectibleTaken)
    (Utilities|FlowControl|Delay 0.8)
    (Actor|DestroyActor)))

(event EventBeginPlay)

(event Collision|EventActorBeginOverlap
  (params (OtherActor :type Actor%20Object%20Reference)))

(event EventTick
  (params (DeltaSeconds :type Float%20%28single-precision%29))
  (bind _scoregottenwidget (Variables|Default|GetScoreGottenWidget))
  (bind _returnvalue (Transformation|GetWorldLocation _scoregottenwidget))
  (if (Variables|/Script/Engine.SceneComponent|GetbVisible (Variables|Default|GetScoreGottenWidget))
    (bind _asbp_third_person_character (Utilities|Casting|CastToBP_ThirdPersonCharacter (Game|GetPlayerCharacter 0)))
    (Transformation|SetWorldRotation _scoregottenwidget (Math|Rotator|MakeRotator 0.0 0.0 (.yaw (Math|Rotator|FindLookatRotation _returnvalue (Transformation|GetWorldLocation (Variables|/Game/ThirdPerson/Blueprints/BP_ThirdPersonCharacter.BP_ThirdPersonCharacter_C|GetFollowCamera _asbp_third_person_character))))) false false)
    (Transformation|SetWorldLocation _scoregottenwidget (+ _returnvalue "0,0,1.400000") false false)))

(fn ConstructionScript)

(fn SpawnMonsterDetection
  (bind _asbp_tpgame_instance (Utilities|Casting|CastToBP_TPGameInstance (Game|GetGameInstance)))
  (bind _outactors (Actor|GetAllActorsOfClass "/Game/ThirdPerson/Blueprints/BP_AIMonsterBase.BP_AIMonsterBase_C"))
  (if (< (Utilities|Array|Length _outactors) 30)
    (if (< (* (Utilities|Array|Length _outactors) (Variables|Default|GetPointSpawnInterval)) (Variables|/Game/ThirdPerson/Blueprints/BP_TPGameInstance.BP_TPGameInstance_C|GetScore _asbp_tpgame_instance))
      (bind _outactors_2 (Actor|GetAllActorsOfClass "/Game/Blueprints/BP_MonSpawnerManager.BP_MonSpawnerManager_C"))
      (for _array_element _outactors_2
        (Default|SpawnatTargetPoint _array_element)))))

(fn CollectibleTaken)